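; BP_SpeedPickup is a pickup that temporarily raises the player's walk speed.
; When a BP_Player overlaps its Sphere, it saves MaxWalkSpeed and adds SpeedAmount.
; After a Delay of Duration, it restores the saved speed and destroys itself.
; The pickup stays active during the delay, so another overlap adds speed again and overwrites the saved value.
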(event `self.Sphere.OnComponentBeginOverlap`
  (params (OverlappedComponent :type "PrimitiveComponent Object Reference") (OtherActor :type "Actor Object Reference") (OtherComp :type "PrimitiveComponent Object Reference") (OtherBodyIndex :type Integer) (bFromSweep :type Boolean) (SweepResult :type "HitResult Structure (by ref)"))
  (bind _asbp_player (cast `/Game/BP_Player` OtherActor))
  (bind _output_get (set `self.PlayerRef` _asbp_player))
  (bind _charactermovement (`Character.CharacterMovement` _output_get))
  (bind _output_get_2 (set `self.OriginalSpeed` (`CharacterMovementComponent.MaxWalkSpeed` _charactermovement)))
  (set `CharacterMovementComponent.MaxWalkSpeed` (+ _output_get_2 (`self.SpeedAmount`)) _charactermovement)
  (`KismetSystemLibrary.Delay` (`self.Duration`))
  (set `CharacterMovementComponent.MaxWalkSpeed` (`self.OriginalSpeed`) (`Character.CharacterMovement` (`self.PlayerRef`)))
  (`self.K2_DestroyActor`))

(fn `UserConstructionScript`)