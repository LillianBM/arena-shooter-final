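; BP_AIEnemy is a shooting enemy that takes damage, awards score on death and respawns.
; On BeginPlay it stores full health and its starting transform, and links itself to its health widget.
; AnyDamage reduces health; on death it increments the player's Score, hides, then spawns a replacement at the start point after a delay and destroys itself.
; ShootAtPlayer fires BP_Projectile toward the player, gated by a cooldown.
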(event `self.ReceiveBeginPlay`
  (`|ExecutionSequence`
    (:`then_0`
      (set `self.Health` (`self.MaxHealth`))
      (bind _output_get (set `self.Respawn Location` (`self.K2_GetActorLocation`)))
      (bind _output_get_2 (set `self.Respawn Rotation` (`self.K2_GetActorRotation`))))
    (:`then_1`
      (bind _aswbp_aihealth (cast `/Game/Blueprints/WBP_AIHealth` (`WidgetComponent.GetUserWidgetObject` (`self.Widget`))))
      (set `/Game/Blueprints/WBP_AIHealth.AIEnemyRef` self _aswbp_aihealth))))

(event `self.ReceiveAnyDamage`
  (params (Damage :type "Float (single-precision)") (DamageType :type "DamageType Object Reference") (InstigatedBy :type "Controller Object Reference") (DamageCauser :type "Actor Object Reference"))
  (bind _returnvalue (- (`self.Health`) Damage))
  (set `self.Health` _returnvalue)
  (`KismetSystemLibrary.PrintString` "AI HIT")
  (if (<= _returnvalue 0.0)
    (`|ExecutionSequence`
      (:`then_0`
        (`self.SetActorHiddenInGame` true)
        (`self.SetActorEnableCollision` false)
        (`KismetSystemLibrary.Delay` 2.0)
        (`|SpawnActorFromClass` "BP_AIEnemy_C" (`KismetMathLibrary.MakeTransform` (stale `self.ReceiveBeginPlay` _output_get) (stale `self.ReceiveBeginPlay` _output_get_2)) "AlwaysSpawn" "MultiplyWithRoot" null null)
        (`self.K2_DestroyActor`))
      (:`then_1`
        (bind _asbp_player (cast `/Game/BP_Player` (`GameplayStatics.GetPlayerCharacter` 0)))
        (set `/Game/BP_Player.Score` (+ (`/Game/BP_Player.Score` _asbp_player) 1) _asbp_player)))))

(event `ShootAtPlayer`
  (bind _returnvalue (`self.K2_GetActorLocation`))
  (if (`self.CanShoot`)
    (set `self.CanShoot` false)
    (`KismetSystemLibrary.PrintString` "AI SHOOT")
    (`|SpawnActorFromClass` "/Game/BP_Projectile.BP_Projectile_C" (`KismetMathLibrary.MakeTransform` (+ (* (`self.GetActorForwardVector`) 100.0) _returnvalue) (`KismetMathLibrary.FindLookAtRotation` _returnvalue (`self.K2_GetActorLocation` (`GameplayStatics.GetPlayerCharacter` 0)))) "Undefined" "MultiplyWithRoot" self null)
    (`KismetSystemLibrary.Delay` 1.0)
    (set `self.CanShoot` true)))

(fn `UserConstructionScript`)